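; BP_RadialBlur is a Blueprint that, going by its name, drives a radial blur effect based on player movement.
; Each Tick checks player pawn 0's speed against a threshold and, while above it, accumulates delta time into CurrentWeight with no clamp.
; At or below the threshold, the weight snaps back to zero, and both branches pass it to SetWeight.
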(event `self.ReceiveTick`
  (params (DeltaSeconds :type "Float (single-precision)"))
  (if (> (`KismetMathLibrary.VSize` (`self.GetVelocity` (`GameplayStatics.GetPlayerPawn` 0))) 100.0)
    (bind _output_get (set `self.CurrentWeight` (+ (`self.CurrentWeight`) DeltaSeconds)))
    (`self.SetWeight` _output_get)
    (else
      (bind _output_get_2 (set `self.CurrentWeight` 0.0))
      (`self.SetWeight` _output_get_2))))

(fn `UserConstructionScript`)