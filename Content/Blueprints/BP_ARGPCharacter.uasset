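; Dual-blade character Blueprint with procedural foot IK, melee hit detection and health feedback.
; Tick line-traces under each foot, feeding ground-aligned rotations and interpolated mesh and effector offsets to the C_SM AnimBP.
; BeginPlay adds the fight HUD, disables blade hitboxes and binds health changes to damage pop-ups and hurt or death sounds.
; Hitbox overlaps apply Atk damage through the attributes component, then disable LeftKatana or RightCollisonBox collision on success.
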(event `self.ReceiveTick`
  (params (DeltaSeconds :type "Float (single-precision)"))
  (bind _animbp (`self.AnimBP`))
  ;[0 0 0] IK实现脚自动抬高
  (bind (_distance _returnvalue) (`self.IK Line Trace` "foot_l" 50.0))
  (set `/Game/Animations/C_SM.Foot Rotation Left` _returnvalue (`self.AnimBP`))
  (bind (_distance_2 _returnvalue_2) (`self.IK Line Trace` "foot_r" 50.0))
  (set `/Game/Animations/C_SM.Foot Rotation Right` _returnvalue_2 (`self.AnimBP`))
  (if (< _distance_2 _distance)
    (set `/Game/Animations/C_SM.Mesh Offset Z` (`KismetMathLibrary.FInterpTo` (`/Game/Animations/C_SM.Mesh Offset Z` (`self.AnimBP`)) _distance_2 (`GameplayStatics.GetWorldDeltaSeconds`) 3.0) _animbp)
    (set `/Game/Animations/C_SM.Effector Location Right` (`KismetMathLibrary.FInterpTo` (`/Game/Animations/C_SM.Effector Location Right` (`self.AnimBP`)) 0.0 (`GameplayStatics.GetWorldDeltaSeconds`) 3.0) _animbp)
    (bind _returnvalue_3 (* (`KismetMathLibrary.Abs` (- _distance_2 _distance)) -1.0))
    (set `/Game/Animations/C_SM.Effector Location Left` (`KismetMathLibrary.FInterpTo` (`/Game/Animations/C_SM.Effector Location Left` (`self.AnimBP`)) _returnvalue_3 (`GameplayStatics.GetWorldDeltaSeconds`) 3.0) _animbp)
    (else
      (set `/Game/Animations/C_SM.Mesh Offset Z` (`KismetMathLibrary.FInterpTo` (`/Game/Animations/C_SM.Mesh Offset Z` (`self.AnimBP`)) _distance (`GameplayStatics.GetWorldDeltaSeconds`) 3.0) _animbp)
      (set `/Game/Animations/C_SM.Effector Location Left` (`KismetMathLibrary.FInterpTo` (`/Game/Animations/C_SM.Effector Location Left` (`self.AnimBP`)) 0.0 (`GameplayStatics.GetWorldDeltaSeconds`) 3.0) _animbp)
      (set `/Game/Animations/C_SM.Effector Location Right` (`KismetMathLibrary.FInterpTo` (`/Game/Animations/C_SM.Effector Location Right` (`self.AnimBP`)) _returnvalue_3 (`GameplayStatics.GetWorldDeltaSeconds`) 3.0) _animbp))))

(event `self.ReceiveBeginPlay`
  (`|ExecutionSequence`
    (:`then_0`
      ;[0 0 0] 设置刀的初始碰撞
      (`PrimitiveComponent.SetCollisionEnabled` (`self.LeftCollisionBox`) "NoCollision")
      (`PrimitiveComponent.SetCollisionEnabled` (`self.RightCollisonBox`) "NoCollision")
      ;[0 0 0] 创建HUD
      (bind _returnvalue (`|CreateWidget` "/Game/UI/Fight_HUD.Fight_HUD_C"))
      (`UserWidget.AddToViewport` _returnvalue 0)
      ;[0 0 0] 获取胶囊体半高
      (bind _asc_sm (cast `/Game/Animations/C_SM` (`SkeletalMeshComponent.GetAnimInstance` (`self.Mesh`))))
      (set `self.AnimBP` _asc_sm)
      (set `self.HalfHeight` (`CapsuleComponent.GetScaledCapsuleHalfHeight` (`self.CapsuleComponent`))))
    (:`then_1`
      (bind _returnvalue_2 (`AttributeComponent.GetAttributes` self))
      (add `AttributeComponent.OnHealthChanged` _returnvalue_2 (delegate `OnHealthChanged_Event`)))))

(event `OnHealthChanged_Event`
  (params (InstigatorActor :type "Actor Object Reference") (OwningComp :type "AttributeComponent Object Reference") (NewValue :type "Float (double-precision)") (Delta :type "Float (double-precision)"))
  (bind _returnvalue (`KismetMathLibrary.Abs` Delta))
  ;[0 0 0] 角色受伤弹出伤害数字
  (if (> NewValue 0.0)
    (if (< Delta 0.0)
      (bind _returnvalue_2 (`|CreateWidget` "/Game/UI/DamagePopUp_Widget.DamagePopUp_Widget_C" null _returnvalue self))
      (`UserWidget.AddToViewport` _returnvalue_2 0)
      (if (> _returnvalue 20.0)
        (`GameplayStatics.SpawnSoundAttached` null (`self.Mesh`) "None" (0.0 0.0 0.0) (struct) "KeepRelativeOffset" false 1.0 1.0 0.0 null null)))
    (else
      (`GameplayStatics.SpawnSoundAttached` null (`self.Mesh`) "None" (0.0 0.0 0.0) (struct) "KeepRelativeOffset" true 1.0 1.0 0.0 null null) ; Attach to mesh so it follows along when ragdolling during death (the capsule remains behind)
    )))

(event `self.LeftCollisionBox.OnComponentBeginOverlap`
  (params (OverlappedComponent :type "PrimitiveComponent Object Reference") (OtherActor :type "Actor Object Reference") (OtherComp :type "PrimitiveComponent Object Reference") (OtherBodyIndex :type Integer) (bFromSweep :type Boolean) (SweepResult :type "HitResult Structure (by ref)"))
  ;[0 0 0] 重叠时对对方施加伤害
  (if (not (== OtherActor self))
    (bind _returnvalue (`AttributeComponent.GetAttributes` OtherActor))
    (`/Engine/EditorBlueprintResources/StandardMacros.IsValid` _returnvalue
      (:`Is Valid`
        (bind _returnvalue_2 (`AttributeComponent.ApplyHealthChange` _returnvalue self (- 0.0 (`self.Atk`))))
        (`KismetSystemLibrary.PrintString` "Hit!")
        ;[0 0 0] 击中目标后取消后续判定
        (if _returnvalue_2
          (`PrimitiveComponent.SetCollisionEnabled` (`self.LeftKatana`) "NoCollision"))))))

(event `self.RightCollisonBox.OnComponentBeginOverlap`
  (params (OverlappedComponent :type "PrimitiveComponent Object Reference") (OtherActor :type "Actor Object Reference") (OtherComp :type "PrimitiveComponent Object Reference") (OtherBodyIndex :type Integer) (bFromSweep :type Boolean) (SweepResult :type "HitResult Structure (by ref)"))
  ;[0 0 0] 重叠时对对方施加伤害
  (if (not (== OtherActor self))
    (bind _returnvalue (`AttributeComponent.GetAttributes` OtherActor))
    (`/Engine/EditorBlueprintResources/StandardMacros.IsValid` _returnvalue
      (:`Is Valid`
        (bind _returnvalue_2 (`AttributeComponent.ApplyHealthChange` _returnvalue self (- 0.0 (`self.Atk`))))
        (`KismetSystemLibrary.PrintString` "Hit!")
        ;[0 0 0] 击中目标后取消后续判定
        (if _returnvalue_2
          (`PrimitiveComponent.SetCollisionEnabled` (`self.RightCollisonBox`) "NoCollision"))))))

(fn `IK Line Trace`
  (params (BoneName :type Name) (TraceDistance :type "Float (double-precision)"))
  (returns (Distance :type "Float (double-precision)") (ReturnValue :type "Rotator Structure"))
  (bind _mesh (`self.Mesh`))
  (bind (_returnvalue_x _returnvalue_y) (`KismetMathLibrary.BreakVector` (`SceneComponent.GetSocketLocation` _mesh BoneName)))
  (bind (_returnvalue_x_2 _returnvalue_y_2 _returnvalue_z) (`KismetMathLibrary.BreakVector` (`SceneComponent.K2_GetComponentLocation` _mesh)))
  (bind _returnvalue (`KismetMathLibrary.MakeVector` _returnvalue_x _returnvalue_y _returnvalue_z))
  (bind (_outhit _returnvalue_2) (`KismetSystemLibrary.LineTraceSingle` :`Start` (+ _returnvalue (`KismetMathLibrary.MakeVector` 0.0 0.0 (`self.HalfHeight`))) :`End` (- _returnvalue (`KismetMathLibrary.MakeVector` 0.0 0.0 TraceDistance)) :`TraceChannel` "TraceTypeQuery1" :`DrawDebugType` "ForOneFrame"))
  (return (`KismetMathLibrary.SelectFloat` (- (`self.HalfHeight`) (`.Distance` (`GameplayStatics.BreakHitResult` _outhit))) 0.0 _returnvalue_2) (`KismetMathLibrary.MakeRotator` (`KismetMathLibrary.DegAtan2` (.y (`.Normal` (`GameplayStatics.BreakHitResult` _outhit))) (.z (`.Normal` (`GameplayStatics.BreakHitResult` _outhit)))) (`KismetMathLibrary.DegAtan2` (.x (`.Normal` (`GameplayStatics.BreakHitResult` _outhit))) (.z (`.Normal` (`GameplayStatics.BreakHitResult` _outhit)))))))

(fn `UserConstructionScript`)