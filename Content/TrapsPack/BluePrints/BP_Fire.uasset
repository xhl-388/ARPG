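; BP_Fire is a fire actor that applies a per-frame health change, named as healing, to RPG characters entering its HealVolume.
; Begin overlap stores the character's attributes and plays the ApplyHeal timeline, whose updates call ApplyHealthChange with HealPerFrame.
; Any actor ending overlap with the whole actor stops the timeline, with no check on which actor left.
; Only the most recently entered character's attributes are held.
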(event `self.ReceiveBeginPlay`
  (add `PrimitiveComponent.OnComponentBeginOverlap` (`self.HealVolume`) (delegate `OnComponentBeginOverlap_Event`))
  (add `self.OnActorEndOverlap` (delegate `OnActorEndOverlap_Event`)))

(event `OnActorEndOverlap_Event` :!signature `self.OnActorEndOverlap`
  (params (OverlappedActor :type "Actor Object Reference") (OtherActor :type "Actor Object Reference"))
  (`Timeline|ApplyHeal` :!via `Stop` :!label _label
    (:`Update`
      (`AttributeComponent.ApplyHealthChange` (stale `OnComponentBeginOverlap_Event` _returnvalue) null (`self.HealPerFrame`)))))

(event `OnComponentBeginOverlap_Event`
  (params (OverlappedComponent :type "PrimitiveComponent Object Reference") (OtherActor :type "Actor Object Reference") (OtherComp :type "PrimitiveComponent Object Reference") (OtherBodyIndex :type Integer) (bFromSweep :type Boolean) (SweepResult :type "HitResult Structure (by ref)"))
  (bind _asarpgcharacter (cast `ARPGCharacter` OtherActor))
  (bind _returnvalue (`AttributeComponent.GetAttributes` _asarpgcharacter))
  (`/Engine/EditorBlueprintResources/StandardMacros.IsValid` _returnvalue
    (:`Is Valid`
      (goto _label))))

(fn `UserConstructionScript`)