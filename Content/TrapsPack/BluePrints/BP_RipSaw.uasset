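; BP_RipSaw is a saw blade trap that damages units overlapping its RotorBlade component.
; On BeginPlay, looping-style motion starts: one timeline slides the blade along local Y after a random delay that staggers instances, while another spins it on roll.
; Overlap begin and end events play and stop the ApplyDamage timeline, whose updates apply DamagePerFrame as a health change through the actor's attributes component.
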(event `self.ReceiveBeginPlay`
  (bind _rotorblade (`self.RotorBlade`))
  (`|ExecutionSequence`
    (:`then_0`
      ;[1 1 1] 添加反复移动动画
      (`KismetSystemLibrary.Delay` (`KismetMathLibrary.Lerp` 3.0 0.0 (`KismetMathLibrary.RandomFloat`)))
      (bind (_direction _move) (`Timeline|Timeline_0`)
        (:`Update`
          (`SceneComponent.K2_SetRelativeLocation` _rotorblade (`KismetMathLibrary.VLerp` (0.0 0.0 4.57) (0.0 220.0 4.57) _move) false false))))
    (:`then_1`
      (bind (_direction_2 _newtrack_0) (`Timeline|Rotor`)
        (:`Update`
          (`SceneComponent.K2_SetRelativeRotation` _rotorblade (`KismetMathLibrary.MakeRotator` _newtrack_0) false false))))
    (:`then_2`
      ;[1 1 1] 对重叠单位施加伤害
      (add `PrimitiveComponent.OnComponentBeginOverlap` (`self.RotorBlade`) (delegate `OnComponentBeginOverlap_Event`))
      (add `PrimitiveComponent.OnComponentEndOverlap` (`self.RotorBlade`) (delegate `OnComponentEndOverlap_Event`)))))

(event `OnComponentEndOverlap_Event`
  (params (OverlappedComponent :type "PrimitiveComponent Object Reference") (OtherActor :type "Actor Object Reference") (OtherComp :type "PrimitiveComponent Object Reference") (OtherBodyIndex :type Integer))
  ;[1 1 1] 对重叠单位施加伤害
  (`Timeline|ApplyDamage` :!via `Stop` :!label _label
    (:`Update`
      (bind _returnvalue (`AttributeComponent.GetAttributes` (stale `OnComponentBeginOverlap_Event` OtherActor)))
      (`/Engine/EditorBlueprintResources/StandardMacros.IsValid` _returnvalue
        (:`Is Valid`
          (`AttributeComponent.ApplyHealthChange` _returnvalue null (`self.DamagePerFrame`)))))))

(event `OnComponentBeginOverlap_Event`
  (params (OverlappedComponent :type "PrimitiveComponent Object Reference") (OtherActor :type "Actor Object Reference") (OtherComp :type "PrimitiveComponent Object Reference") (OtherBodyIndex :type Integer) (bFromSweep :type Boolean) (SweepResult :type "HitResult Structure (by ref)"))
  ;[1 1 1] 对重叠单位施加伤害
  (goto _label))

(fn `UserConstructionScript`)