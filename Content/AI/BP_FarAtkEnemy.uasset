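; BP_FarAtkEnemy is an AI enemy Blueprint, ranged by its name, whose graph handles only damage and death feedback.
; The attribute component's health-change event spawns a damage pop-up widget attached to the enemy for non-lethal losses, adding a sound for major hits only.
; At zero health it plays only a sound, attached to the mesh so it follows the ragdoll rather than the capsule left behind.
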(event `self.AttributeComp.OnHealthChanged`
  (params (InstigatorActor :type "Actor Object Reference") (OwningComp :type "AttributeComponent Object Reference") (NewValue :type "Float (single-precision)") (Delta :type "Float (single-precision)"))
  (bind _returnvalue (`KismetMathLibrary.Abs` Delta))
  (if (> NewValue 0.0)
    (if (< Delta 0.0)
      (bind _returnvalue_2 (`|CreateWidget` "/Game/UI/DamagePopUp_Widget.DamagePopUp_Widget_C" null _returnvalue self))
      (`UserWidget.AddToViewport` _returnvalue_2 0)
      (if (> _returnvalue 20.0)
        (`GameplayStatics.SpawnSoundAttached` null (`self.Mesh`) "None" (0.0 0.0 0.0) (struct) "KeepRelativeOffset" false 1.0 1.0 0.0 null null)))
    (else
      (`GameplayStatics.SpawnSoundAttached` null (`self.Mesh`) "None" (0.0 0.0 0.0) (struct) "KeepRelativeOffset" true 1.0 1.0 0.0 null null) ; Attach to mesh so it follows along when ragdolling during death (the capsule remains behind)
    )))

(fn `UserConstructionScript`)