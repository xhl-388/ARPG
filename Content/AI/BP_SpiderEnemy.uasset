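; Spider enemy character that fights with charge and three-section melee attacks and reacts to health changes.
; The Attack event plays the charge or melee montage, cycling the melee section on each use.
; Overlaps on the left and right plier colliders apply Atk as damage through the other actor's attribute component.
; Health changes spawn damage pop-ups, with attached sounds for major hits and death that follow the ragdolling mesh.
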(event `self.AttributeComp.OnHealthChanged`
  (params (InstigatorActor :type "Actor Object Reference") (OwningComp :type "AttributeComponent Object Reference") (NewValue :type "Float (single-precision)") (Delta :type "Float (single-precision)"))
  (bind _returnvalue (`KismetMathLibrary.Abs` Delta))
  (if (> NewValue 0.0)
    (if (< Delta 0.0)
      (bind _returnvalue_2 (`|CreateWidget` "/Game/UI/DamagePopUp_Widget.DamagePopUp_Widget_C" null _returnvalue self))
      (`UserWidget.AddToViewport` _returnvalue_2 0)
      (if (> _returnvalue 20.0)
        (`GameplayStatics.SpawnSoundAttached` null (`self.Mesh`) "None" (0.0 0.0 0.0) (struct) "KeepRelativeOffset" false 1.0 1.0 0.0 null null)))
    (else
      (`GameplayStatics.SpawnSoundAttached` null (`self.Mesh`) "None" (0.0 0.0 0.0) (struct) "KeepRelativeOffset" true 1.0 1.0 0.0 null null) ; Attach to mesh so it follows along when ragdolling during death (the capsule remains behind)
    )))

(event `self.Attack`
  (params (AttackType :type "EAttackType Enum" :default "Charge"))
  (if (== AttackType (enumliteral `EAttackType` "Charge"))
    (`self.PlayAnimMontage` "/Game/ExampleContent/Enemy_Great_Spider/Animation/AM_Spider_Charge.AM_Spider_Charge")
    (elif (== AttackType (enumliteral `EAttackType` "NAtk"))
      (`self.PlayAnimMontage` "/Game/ExampleContent/Enemy_Great_Spider/Animation/AM_Spider_Melee.AM_Spider_Melee" 1.0 (`KismetStringLibrary.Conv_StringToName` (`KismetStringLibrary.Conv_IntToString` (`self.AtkSection`))))
      (set `self.AtkSection` (mod (+ (`self.AtkSection`) 1) 3))
      (else
        (`KismetSystemLibrary.PrintString` "Invalid Attack Enum")))))

(event `self.LeftPliers.OnComponentBeginOverlap`
  (params (OverlappedComponent :type "PrimitiveComponent Object Reference") (OtherActor :type "Actor Object Reference") (OtherComp :type "PrimitiveComponent Object Reference") (OtherBodyIndex :type Integer) (bFromSweep :type Boolean) (SweepResult :type "HitResult Structure (by ref)"))
  (if (not (== OtherActor self))
    (bind _returnvalue (`AttributeComponent.GetAttributes` OtherActor))
    (`/Engine/EditorBlueprintResources/StandardMacros.IsValid` _returnvalue
      (:`Is Valid`
        (`AttributeComponent.ApplyHealthChange` _returnvalue self (- 0.0 (`self.Atk`)))
        (`KismetSystemLibrary.PrintString` "Hit!")))))

(event `self.RightPliers.OnComponentBeginOverlap`
  (params (OverlappedComponent :type "PrimitiveComponent Object Reference") (OtherActor :type "Actor Object Reference") (OtherComp :type "PrimitiveComponent Object Reference") (OtherBodyIndex :type Integer) (bFromSweep :type Boolean) (SweepResult :type "HitResult Structure (by ref)"))
  (if (not (== OtherActor self))
    (bind _returnvalue (`AttributeComponent.GetAttributes` OtherActor))
    (`/Engine/EditorBlueprintResources/StandardMacros.IsValid` _returnvalue
      (:`Is Valid`
        (`AttributeComponent.ApplyHealthChange` _returnvalue self (- 0.0 (`self.Atk`)))
        (`KismetSystemLibrary.PrintString` "Hit!")))))

(fn `UserConstructionScript`)